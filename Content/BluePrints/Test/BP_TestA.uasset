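; BP_TestA is a test actor that prints boolean values on screen and shows a name on a text render component.
; BeginPlay calls a custom event with false and then true, which prints the flag in green for true or red for false.
; NewFunction_0 forwards an array's first element and a name to that event, which ignores all but the flag.
; The construction script sets the text from MyName.
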(event `self.ReceiveBeginPlay`
  (`self.CustomEvent_0` false)
  (`self.CustomEvent_0` true))

(event `CustomEvent_0`
  (params (NewParam :type Boolean) (NewParam2 :type Byte) (NewParam3 :type Name))
  (`KismetSystemLibrary.PrintString` (`KismetStringLibrary.Conv_BoolToString` NewParam) true false (`KismetMathLibrary.SelectColor` (struct :`G` 1.0 :`B` 0.25 :`A` 1.0) (struct :`R` 1.0 :`G` 0.124938 :`B` 0.134885 :`A` 1.0) NewParam) 5.0))

(event `self.ReceiveTick`
  (params (DeltaSeconds :type "Float (single-precision)")))

(fn `NewFunction_0`
  (params (InName :type Name) (InArray :type "Array of Boolean"))
  (`self.CustomEvent_0` (`|GetArrayItem` InArray) 0 InName))

(fn `UserConstructionScript`
  (`TextRenderComponent.K2_SetText` (`self.TextRender`) (`|FormatText` (`KismetTextLibrary.Conv_NameToText` (`self.MyName`)))))