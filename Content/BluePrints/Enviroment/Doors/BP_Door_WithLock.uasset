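; Door Blueprint that extends a parent door with a lock, opening only while unlocked and showing its state on a red/green indicator light.
; Interact toggles an unlocked door, or checks the overlapping actor's backpack component for all required quest items, calling item removal on matches and Unlock when all are found.
; Lock and Unlock change state only when the required-key list is empty, while SwitchLock toggles it unconditionally.
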(event `self.OpenDoor`
  (if (not (`self.IsDoorLocked`))
    (`parent.OpenDoor`)))

(event `self.CloseDoor`
  (`parent.CloseDoor`))

(fn `Interact`
  (returns (Success :type Boolean))
  (locals (l_ItemInrement :type Integer :default 0) (l_Backpack :type "/Game/BluePrints/Components/BP_BackpackComponent Object Reference") (L_ItemName :type Name))
  (if (`self.IsReadyToInteract`)
    (if (not (`self.IsDoorLocked`))
      (if (`self.IsDoorOpen`)
        (`self.CloseDoor`)
        (return true)
        (else
          (`self.OpenDoor`)
          (return true)))
      (elif (`KismetArrayLibrary.Array_IsValidIndex` (`self.NeededKeysName`))
        (bind _overlappedactor (`self.OverlappedActor`)
          (:`then`
            (bind _returnvalue (`self.GetComponentByClass` _overlappedactor "/Game/BluePrints/Components/BP_BackpackComponent.BP_BackpackComponent_C"))
            (`/Engine/EditorBlueprintResources/StandardMacros.IsValid` _returnvalue
              (:`Is Valid`
                (set `local.l_Backpack` _returnvalue)
                (for _array_element (`self.NeededKeysName`)
                  (if (`BlueprintSetLibrary.Set_Contains` (`/Game/BluePrints/Components/BP_BackpackComponent.QuestItems` (`local.l_Backpack`)) _array_element)
                    (`/Engine/EditorBlueprintResources/StandardMacros.IncrementInt` (`local.l_ItemInrement`)
                      (:`  `
                        ;[1 1 1] if you want to remove item from inventory
                        (`/Game/BluePrints/Components/BP_BackpackComponent.RemoveQuestItem` (`local.l_Backpack`) (`local.L_ItemName`))))))
                (if (== (`local.l_ItemInrement`) (`KismetArrayLibrary.Array_Length` (`self.NeededKeysName`)))
                  (`self.Unlock`)
                  (else
                    (return true))))
              (:`Is Not Valid`
                (return true))))
          (:`else`
            (return true)))
        (else
          (return true))))
    (else
      (return false))))

(fn `Lock`
  (if (not (`KismetArrayLibrary.Array_IsValidIndex` (`self.NeededKeysName`)))
    (set `self.IsDoorLocked` true)
    (`self.UpdateDoorLockIndication`)))

(fn `SwitchLock`
  (set `self.IsDoorLocked` (not (`self.IsDoorLocked`)))
  (`self.UpdateDoorLockIndication`))

(fn `Unlock`
  (if (not (`KismetArrayLibrary.Array_IsValidIndex` (`self.NeededKeysName`)))
    (set `self.IsDoorLocked` false)
    (`self.UpdateDoorLockIndication`)))

(fn `UpdateDoorLockIndication`
  (`LightComponent.SetLightColor` (`self.PointLightLockIndicator`) (`KismetMathLibrary.SelectColor` (struct :`R` 1.0 :`G` 0.008232 :`A` 1.0) (struct :`G` 0.651042 :`B` 0.063616 :`A` 1.0) (`self.IsDoorLocked`)) true))

(fn `UserConstructionScript`
  (`parent.UserConstructionScript`)
  (`self.UpdateDoorLockIndication`))